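; BP_Piece is a game piece actor whose static mesh is tinted with the primary color of its PlayerCore.
; The construction script creates a dynamic material instance for the mesh and sets its Color parameter from that color.
; A RepNotify on PlayerCore reapplies the color to the stored instance, so the tint follows changes to the replicated reference.
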(event EventOnRepPlayerCore
  (Rendering|Material|SetVectorParameterValue (Variables|Default|GetColorMaterialInstance) "Color" (Math|Conversions|ToLinearColor(Color) (Variables|/Script/Ludo.PlayerCore|GetPrimaryColor (Variables|Default|GetPlayerCore))) :!class /Script/Engine.MaterialInstanceDynamic)
  (Rendering|Material|SetMaterial (Variables|Default|GetStaticMesh) 0 (Variables|Default|GetColorMaterialInstance)))

(fn ConstructionScript
  (bind _returnvalue (Rendering|Material|CreateDynamicMaterialInstance (Variables|Default|GetStaticMesh) 0 0 "None" :!class /Script/Engine.PrimitiveComponent))
  (bind _output_get (Variables|Default|SetColorMaterialInstance _returnvalue))
  (Rendering|Material|SetVectorParameterValue _output_get "Color" (Math|Conversions|ToLinearColor(Color) (Variables|/Script/Ludo.PlayerCore|GetPrimaryColor (Variables|Default|GetPlayerCore))) :!class /Script/Engine.MaterialInstanceDynamic)
  (Rendering|Material|SetMaterial (Variables|Default|GetStaticMesh) 0 (Variables|Default|GetColorMaterialInstance)))