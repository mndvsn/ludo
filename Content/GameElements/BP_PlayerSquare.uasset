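; BP_PlayerSquare is a game-element actor whose mesh displays the primary color of its PlayerCore.
; The construction script creates a dynamic instance of M_FilledCircle, tints it with that color and applies it to the mesh.
; SetHighlight switches the Color parameter between a fixed magenta and the player's color, while UpdatePlayerCore reapplies the player's color.
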(event EventBeginPlay)

(event Collision|EventActorBeginOverlap
  (params (OtherActor :type Actor%20Object%20Reference)))

(event EventTick
  (params (DeltaSeconds :type Float%20%28single-precision%29)))

(event EventSetHighlight
  (params (Highlighted :type Boolean))
  (bind _materialinstance (Variables|Default|GetMaterialInstance))
  (bind _staticmesh (Variables|Default|GetStaticMesh))
  (if Highlighted
    (Rendering|Material|SetVectorParameterValue _materialinstance "Color" (Utilities|Struct|MakeLinearColor 0.7 0.0 0.7 1.0) :!class /Script/Engine.MaterialInstanceDynamic)
    (Rendering|Material|SetMaterial _staticmesh 0 _materialinstance)
    (else
      (Rendering|Material|SetVectorParameterValue _materialinstance "Color" (Math|Conversions|ToLinearColor(Color) (.PrimaryColor (Utilities|Struct|BreakPlayerCore (Variables|Default|GetPlayerCore)))) :!class /Script/Engine.MaterialInstanceDynamic)
      (Rendering|Material|SetMaterial _staticmesh 0 _materialinstance))))

(event EventUpdatePlayerCore
  (bind _materialinstance (Variables|Default|GetMaterialInstance))
  (Rendering|Material|SetVectorParameterValue _materialinstance "Color" (Math|Conversions|ToLinearColor(Color) (Utilities|Struct|BreakPlayerCore (Variables|Default|GetPlayerCore))) :!class /Script/Engine.MaterialInstanceDynamic)
  (Rendering|Material|SetMaterial (Variables|Default|GetStaticMesh) 0 _materialinstance))

(fn ConstructionScript
  (bind _returnvalue (Rendering|Material|CreateDynamicMaterialInstance (Variables|Default|GetStaticMesh) 0 "/Game/Objects/M_FilledCircle.M_FilledCircle" "None" :!class /Script/Engine.PrimitiveComponent))
  (bind _output_get (Variables|Default|SetMaterialInstance _returnvalue))
  (Rendering|Material|SetVectorParameterValue _output_get "Color" (Math|Conversions|ToLinearColor(Color) (.PrimaryColor (Utilities|Struct|BreakPlayerCore (Variables|Default|GetPlayerCore)))) :!class /Script/Engine.MaterialInstanceDynamic)
  (Rendering|Material|SetMaterial (Variables|Default|GetStaticMesh) 0 _output_get))