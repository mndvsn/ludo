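; BP_Square is a game element with a Cylinder mesh that can be visually highlighted.
; The construction script creates a dynamic material instance from M_Debug on the mesh and caches its Color parameter as the default.
; The SetHighlight event switches that Color parameter between a fixed orange and the cached default, then reapplies the material to the mesh.
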(event EventBeginPlay)

(event Collision|EventActorBeginOverlap
  (params (OtherActor :type Actor%20Object%20Reference)))

(event EventTick
  (params (DeltaSeconds :type Float%20%28single-precision%29)))

(event EventSetHighlight
  (params (Highlighted :type Boolean))
  (bind _material (Variables|Default|GetMaterial))
  (bind _cylinder (Variables|Default|GetCylinder))
  (if Highlighted
    (Rendering|Material|SetVectorParameterValue _material "Color" (Utilities|Struct|MakeLinearColor 1.0 0.4 0.0 1.0) :!class /Script/Engine.MaterialInstanceDynamic)
    (Rendering|Material|SetMaterial _cylinder 0 _material)
    (else
      (Rendering|Material|SetVectorParameterValue _material "Color" (Variables|Default|GetDefaultColor) :!class /Script/Engine.MaterialInstanceDynamic)
      (Rendering|Material|SetMaterial _cylinder 0 _material))))

(fn ConstructionScript
  (bind _returnvalue (Rendering|Material|CreateDynamicMaterialInstance (Variables|Default|GetCylinder) 0 "/Game/Objects/M_Debug.M_Debug" "None" :!class /Script/Engine.PrimitiveComponent))
  (bind _output_get (Variables|Default|SetMaterial _returnvalue))
  (bind _returnvalue_2 (Rendering|Material|GetVectorParameterValue _output_get "Color" :!class /Script/Engine.MaterialInstanceDynamic))
  (Variables|Default|SetDefaultColor _returnvalue_2))