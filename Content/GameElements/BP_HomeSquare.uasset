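; BP_HomeSquare is a player's home square on the board, tinted with the primary color of its PlayerCore.
; The construction script creates a dynamic M_Piece material instance on mesh slot 1, sets its Color parameter and also applies it to slot 0.
; SetHighlight switches that Color between a fixed orange and the player's primary color, then reapplies the material to slot 1.
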(event EventBeginPlay)

(event Collision|EventActorBeginOverlap
  (params (OtherActor :type Actor%20Object%20Reference)))

(event EventTick
  (params (DeltaSeconds :type Float%20%28single-precision%29)))

(event EventSetHighlight
  (params (Highlighted :type Boolean))
  (bind _material (Variables|Default|GetMaterial))
  (bind _staticmesh (Variables|Default|GetStaticMesh))
  (if Highlighted
    (Rendering|Material|SetVectorParameterValue _material "Color" (Utilities|Struct|MakeLinearColor 1.0 0.4 0.0 1.0) :!class /Script/Engine.MaterialInstanceDynamic)
    (Rendering|Material|SetMaterial _staticmesh 1 _material)
    (else
      (Rendering|Material|SetVectorParameterValue _material "Color" (Math|Conversions|ToLinearColor(Color) (Variables|/Script/Ludo.PlayerCore|GetPrimaryColor (Variables|Default|GetPlayerCore))) :!class /Script/Engine.MaterialInstanceDynamic)
      (Rendering|Material|SetMaterial _staticmesh 1 _material))))

(fn ConstructionScript
  (bind _returnvalue (Rendering|Material|CreateDynamicMaterialInstance (Variables|Default|GetStaticMesh) 1 "/Game/Objects/M_Piece.M_Piece" "None" :!class /Script/Engine.PrimitiveComponent))
  (bind _output_get (Variables|Default|SetMaterial _returnvalue))
  (Rendering|Material|SetVectorParameterValue _output_get "Color" (Math|Conversions|ToLinearColor(Color) (Variables|/Script/Ludo.PlayerCore|GetPrimaryColor (Variables|Default|GetPlayerCore))) :!class /Script/Engine.MaterialInstanceDynamic)
  (Rendering|Material|SetMaterial (Variables|Default|GetStaticMesh) 0 _output_get))